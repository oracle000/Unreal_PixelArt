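; Player character with a flipbook sprite that moves, jumps, attacks, blocks and plays a death animation from Enhanced Input actions.
; BeginPlay adds the default mapping context, and each action swaps the sprite's flipbook, with movement also flipping sprite rotation by direction.
; IsJumping gates movement, attack and repeat jumps, while IsAttacking blocks repeat attacks.
; Landing is detected by a Delay loop polling vertical velocity until zero, then restoring looping idle.
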(event Input|EnhancedActionEvents|EnhancedInputActionIA_Movement
  (params (ActionValue :type Float%20%28double-precision%29) (ElapsedSeconds :type Float%20%28double-precision%29) (TriggeredSeconds :type Float%20%28double-precision%29) (InputAction :type Input%20Action%20Object%20Reference :default "/Game/Blueprint/IA_Movement.IA_Movement"))
  (:Triggered
    (if (not (Variables|Default|GetIsJumping))
      (Pawn|Input|AddMovementInput (Transformation|GetActorForwardVector) ActionValue false)
      (Sprite|SetFlipbook (Variables|Default|GetSprite) "/Game/Player_Anim/FB_Run.FB_Run")
      (if (> ActionValue 0.0)
        (Transformation|SetWorldRotation (Variables|Default|GetSprite) "0, 0, 0" false false)
        (else
          (Transformation|SetWorldRotation (Variables|Default|GetSprite) "0.000000,-180.000000,0.000000" false false)))))
  (:Completed
    (Sprite|SetFlipbook (Variables|Default|GetSprite) "/Game/Player_Anim/FB_Idle.FB_Idle")))

(event Input|EnhancedActionEvents|EnhancedInputActionIA_Jump
  (params (ActionValue :type Boolean) (ElapsedSeconds :type Float%20%28double-precision%29) (TriggeredSeconds :type Float%20%28double-precision%29) (InputAction :type Input%20Action%20Object%20Reference :default "/Game/Blueprint/IA_Jump.IA_Jump"))
  (bind _sprite (Variables|Default|GetSprite))
  (:Triggered
    (if (not (Variables|Default|GetIsJumping))
      (Variables|Default|SetIsJumping true)
      (Character|Jump)
      (Components|Timeline|SetLooping _sprite false)
      (Sprite|SetFlipbook _sprite "/Game/Player_Anim/FB_Jump.FB_Jump")
      (Utilities|FlowControl|Delay 0.2)
      (if (== (.Z (Math|Vector|BreakVector (Transformation|GetVelocity))) 0.0) :!label _label
        (Components|Timeline|SetLooping _sprite true)
        (Audio|Components|Audio|Play _sprite)
        (Sprite|SetFlipbook _sprite "/Game/Player_Anim/FB_Idle.FB_Idle")
        (Variables|Default|SetIsJumping false)
        (else
          (Utilities|FlowControl|Delay 0.2)
          (goto _label))))))

(event Input|EnhancedActionEvents|EnhancedInputActionIA_Attack
  (params (ActionValue :type Boolean) (ElapsedSeconds :type Float%20%28double-precision%29) (TriggeredSeconds :type Float%20%28double-precision%29) (InputAction :type Input%20Action%20Object%20Reference :default "/Game/Blueprint/IA_Attack.IA_Attack"))
  (bind _sprite (Variables|Default|GetSprite))
  (:Triggered
    (if (not (Variables|Default|GetIsJumping))
      (if (not (Variables|Default|GetIsAttacking))
        (Sprite|SetFlipbook _sprite "/Game/Player_Anim/FB_Attack1.FB_Attack1")
        (Variables|Default|SetIsAttacking true))))
  (:Completed
    (Utilities|FlowControl|Delay 0.4)
    (Sprite|SetFlipbook _sprite "/Game/Player_Anim/FB_Idle.FB_Idle")
    (Variables|Default|SetIsAttacking false)))

(event Input|EnhancedActionEvents|EnhancedInputActionIA_Dead
  (params (ActionValue :type Boolean) (ElapsedSeconds :type Float%20%28double-precision%29) (TriggeredSeconds :type Float%20%28double-precision%29) (InputAction :type Input%20Action%20Object%20Reference :default "/Game/Blueprint/IA_Dead.IA_Dead"))
  (:Triggered
    (Sprite|SetFlipbook (Variables|Default|GetSprite) "/Game/Player_Anim/FB_Dead.FB_Dead")
    (Utilities|FlowControl|Delay 0.5)
    (Sprite|SetFlipbook (Variables|Default|GetSprite) "/Game/Player_Anim/FB_Dead_End.FB_Dead_End")))

(event Input|EnhancedActionEvents|EnhancedInputActionIA_Block
  (params (ActionValue :type Boolean) (ElapsedSeconds :type Float%20%28double-precision%29) (TriggeredSeconds :type Float%20%28double-precision%29) (InputAction :type Input%20Action%20Object%20Reference :default "/Game/Blueprint/IA_Block.IA_Block"))
  (bind _sprite (Variables|Default|GetSprite))
  (:Triggered
    (Sprite|SetFlipbook _sprite "/Game/Player_Anim/FB_Block.FB_Block")
    (Sprite|SetFlipbook _sprite "/Game/Player_Anim/FB_Block_End.FB_Block_End"))
  (:Completed
    (Sprite|SetFlipbook (Variables|Default|GetSprite) "/Game/Player_Anim/FB_Idle.FB_Idle")))

(event EventBeginPlay
  (bind _asbp_player_controller (Utilities|Casting|CastToBP_PlayerController (Pawn|GetController)))
  (Input|AddMappingContext (PlayerController|LocalPlayerSubsystems|GetEnhancedInputLocalPlayerSubsystem _asbp_player_controller) "/Game/Blueprint/IMC_Default.IMC_Default" 0 "(bIgnoreAllPressedKeysUntilRelease=True,bForceImmediately=False)"))

(fn ConstructionScript)

(fn MySampleFunction
  (Development|PrintText (Utilities|Text|ToText(Integer) 0)))