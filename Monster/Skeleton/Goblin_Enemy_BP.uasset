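; Goblin_Enemy_BP is a Paper2D enemy character that uses skeleton flipbooks despite its goblin name.
; Each Tick runs an animation update that switches the sprite between walk and idle flipbooks based on whether its movement velocity is non-zero.
; A movement update is also called every Tick but is an empty stub, so the Blueprint contains no movement or AI logic of its own.
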(event Custom|Animation%20Update
  (Sprite|SetFlipbook (Variables|Default|GetSprite) (select (> (Math|Vector|VectorLength (Variables|/Script/Engine.MovementComponent|GetVelocity (Variables|Character|GetCharacterMovement))) 0.0) (Variables|Default|GetSkeleton_Walk_FB) (Variables|Default|GetSkeleton_Idle_FB))))

(event Custom|Movement%20Update)

(event EventBeginPlay)

(event EventTick
  (params (DeltaSeconds :type Float%20%28single-precision%29))
  (CallFunction|AnimationUpdate)
  (CallFunction|MovementUpdate))

(fn ConstructionScript)